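; Player controller for a MegaJam game that turns look and movement axis inputs into control of the player character.
; Look axes add controller pitch and yaw input to player character 0.
; Horizontal and vertical movement axes add movement input along the controller's own right and forward vectors, rather than the character's.
; BeginPlay, Tick and the construction script are empty.
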(event EventBeginPlay)

(event EventTick
  (params (DeltaSeconds :type Float%20%28single-precision%29)))

(event Input|AxisEvents|InputAxisHorizontalMovement
  (params (AxisValue :type Float%20%28single-precision%29))
  ;[1 1 1] WASD Control
  (Pawn|Input|AddMovementInput (Game|GetPlayerCharacter 0) (Transformation|GetActorRightVector) AxisValue false))

(event Input|AxisEvents|InputAxisVerticalMovement
  (params (AxisValue :type Float%20%28single-precision%29))
  ;[1 1 1] WASD Control
  (Pawn|Input|AddMovementInput (Game|GetPlayerCharacter 0) (Transformation|GetActorForwardVector) AxisValue false))

(event Input|AxisEvents|InputAxisLookUp
  (params (AxisValue :type Float%20%28single-precision%29))
  ;[1 1 1] Rotation Control
  (Pawn|Input|AddControllerPitchInput (Game|GetPlayerCharacter 0) AxisValue))

(event Input|AxisEvents|InputAxisLookRight
  (params (AxisValue :type Float%20%28single-precision%29))
  ;[1 1 1] Rotation Control
  (Pawn|Input|AddControllerYawInput (Game|GetPlayerCharacter 0) AxisValue))

(fn ConstructionScript)